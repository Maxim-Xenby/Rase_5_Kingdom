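; Actor component that tracks a weapon's ammo count.
; On BeginPlay it fills current ammo to the maximum.
; It exposes a subtract function that clamps the count between zero and the maximum, and a check that reports whether enough ammo remains for a given amount.
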(event `self.ReceiveBeginPlay`
  (set `self.Curent_Ammo` (`self.Max_Ammo`)))

(fn `Chek_Ammo`
  (params (Value :type Integer :default 1))
  (returns (ReturnValue :type Boolean))
  (return (>= (`self.Curent_Ammo`) Value)))

(fn `Sudstruct_ammo`
  (params (VAlue :type Integer :default 1))
  (set `self.Curent_Ammo` (`KismetMathLibrary.Clamp` (- (`self.Curent_Ammo`) VAlue) 0 (`self.Max_Ammo`))))