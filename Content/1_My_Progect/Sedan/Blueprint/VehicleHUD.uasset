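; Vehicle HUD Blueprint that creates the player's UI_Player widget on BeginPlay and draws a speed readout on screen.
; DrawHUD casts the owning pawn to Man_Car and draws its SpeedDisplayString only while IsInCar is false.
; Text position scales with screen size relative to a 720p layout, and font scale follows the height ratio.
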(event `self.ReceiveDrawHUD`
  (params (SizeX :type Integer) (SizeY :type Integer))
  (bind _hudyratio (`self.HUDYRatio`))
  ;[1 1 1] Расположения для 720p
  (bind _asman_car (cast `/Game/1_My_Progect/Sedan/Man_Car` (`self.GetOwningPawn`)))
  (if (not (`/Game/1_My_Progect/Sedan/Man_Car.IsInCar` _asman_car))
    (`|ExecutionSequence`
      (:`then_0`
        (set `self.HUDXRatio` (/ (`KismetMathLibrary.Conv_IntToDouble` SizeX) 1280.0)))
      (:`then_1`
        (set `self.HUDYRatio` (/ (`KismetMathLibrary.Conv_IntToDouble` SizeY) 720.0)))
      (:`then_2`
        ;[1 1 1] Вывод скорости
        (bind _asman_car_2 (cast `/Game/1_My_Progect/Sedan/Man_Car` (`self.GetOwningPawn`)))
        (`self.DrawText` (`/Game/1_My_Progect/Sedan/Man_Car.Speed Display String` _asman_car_2) (struct :`R` 1.0 :`G` 1.0 :`B` 1.0 :`A` 1.0) (* 805.0 (`self.HUDXRatio`)) (* 455.0 _hudyratio) "/Engine/EngineFonts/RobotoDistanceField.RobotoDistanceField" (* 1.4 _hudyratio))))))

(event `self.ReceiveBeginPlay`
  ;[1 1 1] Создание интерфейса игрока
  (bind _returnvalue (`|CreateWidget` "/Game/1_My_Progect/UI/UI_Player.UI_Player_C" (`GameplayStatics.GetPlayerController` 0)))
  (`UserWidget.AddToViewport` _returnvalue 0))

(fn `UserConstructionScript`)