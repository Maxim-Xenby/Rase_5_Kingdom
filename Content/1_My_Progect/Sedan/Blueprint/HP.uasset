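; HP Blueprint for the Sedan that tracks health and nitro, both filled to their maximums on BeginPlay.
; Damage subtracts from health and fires the OnDead dispatcher through a DoOnce when health reaches zero.
; AddHeal adds health without capping it at the maximum, while AddNitro clamps to MaxNitro.
; Despite its getter name, GetNitro consumes one unit of nitro per call, clamped at zero.
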(event `self.ReceiveBeginPlay`
  (`|ExecutionSequence`
    (:`then_0`
      (set `self.Current_HP` (`self.Max_HP`)))
    (:`then_1`
      (set `self.Current_Nitro` (`self.Max_Nitro`)))))

(fn `Add Heal`
  (params (Add :type "Float (double-precision)" :default 0.0))
  (set `self.Current_HP` (+ Add (`self.Current_HP`)))
  (return))

(fn `Add_Nitro`
  (params (Add :type "Float (double-precision)" :default 1.0))
  (set `self.Current_Nitro` (`KismetMathLibrary.FClamp` (+ Add (`self.Current_Nitro`)) 0.0 (`self.Max_Nitro`)))
  (return))

(fn `Damage`
  (params (Damage :type "Float (double-precision)"))
  (set `self.Current_HP` (- (`self.Current_HP`) Damage))
  (if (<= (`self.Current_HP`) 0.0)
    (`/Engine/EditorBlueprintResources/StandardMacros.DoOnce` false
      (:`Completed`
        (`self.On Dead`)))))

(fn `Get Heal`
  (returns (Get :type "Float (double-precision)"))
  (return (`self.Current_HP`)))

(fn `Get_Nitro`
  (set `self.Current_Nitro` (`KismetMathLibrary.FClamp` (- (`self.Current_Nitro`) 1.0) 0.0 (`self.Max_Nitro`)))
  (return))

(fn `Is Dead`
  (returns (Yes :type Boolean))
  (return (<= (`self.Current_HP`) 0.0)))